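; BP_MAZE is a procedural maze generator that builds seeded path and dead-end tile sets in its construction script.
; GenerateMaze runs a randomized depth-first carve, recursing two cells at a time and backtracking to join cells through bridge tiles.
; SpawnMazeMeshes turns those sets into instanced floor, end-floor, wall and raised tiles through InstanceManager.
; The construction script clears old instances and evens Size, but its spawning calls are disconnected.
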(fn `AddNeighborLoc`
  (params (Size :type "IntPoint Structure (by ref)") (RandStream :type "RandomStream Structure (by ref)") (CurrentLoc :type "IntPoint Structure (by ref)") (PathTiles :type "Set of IntPoint Structure (by ref)") (BridgeTiles :type "Set of IntPoint Structure (by ref)") (ToCheck :type "Set of IntPoint Structure (by ref)") (EndPaths :type "Set of IntPoint Structure (by ref)"))
  (locals (NeighborIndex :type Integer))
  (bind (_floor _bridge) (`self.GetNeighborAndBridge` (`local.CurrentLoc`) (`local.NeighborIndex`)))
  (bind _returnvalue (+ (`local.NeighborIndex`) 1))
  (set `local.NeighborIndex` (`KismetMathLibrary.RandomIntegerInRangeFromStream` (`local.RandStream`) 0 3))
  (if (`self.CheckIsValidLoc` (`self.GetNeighborAndBridge` (`local.CurrentLoc`) (`local.NeighborIndex`)) (`local.Size`) (`local.PathTiles`) (`local.BridgeTiles`)) :!label _label
    (`BlueprintSetLibrary.Set_Add` (`local.PathTiles`) _floor)
    (`BlueprintSetLibrary.Set_Add` (`local.BridgeTiles`) _bridge)
    (`BlueprintSetLibrary.Set_Add` (`local.ToCheck`) _floor)
    (`self.AddNeighborLoc` (`local.Size`) (`local.RandStream`) _floor (`local.PathTiles`) (`local.BridgeTiles`) (`local.ToCheck`) (`local.EndPaths`))
    (else
      (`/Game/MazeComponents/Blueprints/CustomMacLibrary.DoN+` 4
        (:`Exit`
          (set `local.NeighborIndex` (`KismetMathLibrary.SelectInt` 0 _returnvalue (>= _returnvalue 4)))
          (goto _label))
        (:`OverNth`
          (bind _count (`self.GetNeighborCount` (`local.CurrentLoc`) (`local.PathTiles`)))
          (if (== _count 1)
            (`BlueprintSetLibrary.Set_Add` (`local.EndPaths`) (`local.CurrentLoc`))))))))

(fn `Backtrack`
  (params (`Current Tile` :type "IntPoint Structure (by ref)") (ToCheck :type "Set of IntPoint Structure (by ref)") (BridgeTiles :type "Set of IntPoint Structure (by ref)") (PathTiles :type "Set of IntPoint Structure (by ref)"))
  (bind _result (`BlueprintSetLibrary.Set_ToArray` ToCheck))
  (bind _output (`|GetArrayItem` _result (`KismetArrayLibrary.Array_LastIndex` _result)))
  (`|VariableSetRef` (`local.Current Tile`) _output)
  (`BlueprintSetLibrary.Set_Remove` (`local.ToCheck`) _output)
  (bind _result_2 (`BlueprintSetLibrary.Set_ToArray` (`local.BridgeTiles`)))
  (bind _output_2 (`|GetArrayItem` _result_2 (`KismetArrayLibrary.Array_LastIndex` _result_2)))
  (`BlueprintSetLibrary.Set_Add` (`local.PathTiles`) _output_2)
  (`BlueprintSetLibrary.Set_Remove` (`local.BridgeTiles`) _output_2))

(fn `Generate Maze`
  (params (SIze :type "IntPoint Structure") (Seed :type Integer))
  (returns (`Path Tiles Out` :type "Set of IntPoint Structure") (`End Paths Out` :type "Set of IntPoint Structure"))
  (locals (RandStream :type "RandomStream Structure") (`L Size` :type "IntPoint Structure") (StartingLoc :type "IntPoint Structure") (CurrentLoc :type "IntPoint Structure") (`Path Tiles` :type "Set of IntPoint Structure") (BridgeTiles :type "Set of IntPoint Structure") (ToCheck :type "Set of IntPoint Structure") (`End Paths` :type "Set of IntPoint Structure"))
  (`KismetMathLibrary.SetRandomStreamSeed` (`local.RandStream`) Seed)
  (set `local.L Size` SIze)
  (bind _output_get (set `local.StartingLoc` (`self.GetRandomLocInBounds` (`local.L Size`) (`local.RandStream`))))
  (set `local.CurrentLoc` _output_get)
  (`self.AddNeighborLoc` (`local.L Size`) (`local.RandStream`) (`local.CurrentLoc`) (`local.Path Tiles`) (`local.BridgeTiles`) (`local.ToCheck`) (`local.End Paths`) :!label _label)
  (if (> (`BlueprintSetLibrary.Set_Length` (`local.ToCheck`)) 0)
    (`self.Backtrack` (`local.CurrentLoc`) (`local.ToCheck`) (`local.BridgeTiles`) (`local.Path Tiles`))
    (goto _label)
    (else
      (return (`local.Path Tiles`) (`local.End Paths`)))))

(fn `GetNeighborCount`
  (params (CurrentLoc :type "IntPoint Structure (by ref)") (PathTiles :type "Set of IntPoint Structure (by ref)"))
  (returns (Count :type Integer))
  (locals (Counter :type Integer))
  (for _array_element (`self.GetNeighborLoc` CurrentLoc 1)
    (if (`BlueprintSetLibrary.Set_Contains` (`local.PathTiles`) _array_element)
      (`/Engine/EditorBlueprintResources/StandardMacros.IncrementInt` (`local.Counter`))))
  (return (`local.Counter`)))

(fn `SpawnMazeMeshes`
  (locals (LoopLoc :type "IntPoint Structure") (LoopIndex :type Integer) (SegmentIndex :type "Array of Boolean"))
  (bind (_size_x _size_y) (break `IntPoint` (`self.Size`)))
  (for _index (range (+ _size_x 1))
    (for _index_2 (range (+ _size_y 1))
      (set `local.LoopLoc` (make `IntPoint` _index_2 _index))
      (if (`BlueprintSetLibrary.Set_Contains` (`self.Path Tiles GM`) (`local.LoopLoc`))
        (message `/Game/MazeComponents/Blueprints/BPI_InstanceManager.AddNewMeshInstance` (`self.InstanceManager`) (select `bool` (`BlueprintSetLibrary.Set_Contains` (`self.End Paths GM`) (`local.LoopLoc`)) :`false` "/Game/MazeComponents/Blueprints/Floor_400x400.Floor_400x400" :`true` "/Game/MazeComponents/Blueprints/End_Floor_400x400.End_Floor_400x400" :!type "StaticMesh Object Reference") (`self.BuildTileLoc` (`local.LoopLoc`)))
        (for (_array_element _array_index) (`self.GetNeighborLoc` (`local.LoopLoc`) 1)
          (set `local.LoopIndex` _array_index)
          (bind _returnvalue (`BlueprintSetLibrary.Set_Contains` (`self.Path Tiles GM`) _array_element))
          (`KismetArrayLibrary.Array_Set` (`local.SegmentIndex`) (`local.LoopIndex`) _returnvalue true)
          (if (not _returnvalue)
            (message `/Game/MazeComponents/Blueprints/BPI_InstanceManager.AddNewMeshInstance` (`self.InstanceManager`) "/Game/StarterContent/Architecture/Wall_400x400.Wall_400x400" (`self.BuildTileLoc` (`local.LoopLoc`) 0.0 (`local.LoopIndex`)))))
        (else
          (message `/Game/MazeComponents/Blueprints/BPI_InstanceManager.AddNewMeshInstance` (`self.InstanceManager`) "/Game/MazeComponents/Blueprints/Floor_400x400.Floor_400x400" (`self.BuildTileLoc` (`local.LoopLoc`) 800.0)))))))

(fn `UserConstructionScript`
  (bind (_size_x _size_y) (break `IntPoint` (`self.Size`)))
  (message `/Game/MazeComponents/Blueprints/BPI_InstanceManager.RemoveAllInstances` (`self.InstanceManager`))
  (set `self.Size` (make `IntPoint` (* (/ _size_x 2) 2) (* (/ _size_y 2) 2)))
  (bind (_path_tiles_out _end_paths_out) (`self.Generate Maze` (`self.Size`) (`self.Seed`)))
  (set `self.Path Tiles GM` _path_tiles_out)
  (set `self.End Paths GM` _end_paths_out))