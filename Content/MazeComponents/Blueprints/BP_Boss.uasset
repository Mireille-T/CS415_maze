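; BP_Boss is a boss enemy that shoots at the player and is defeated by gathering collectibles.
; When PawnSensing sees the player character, it snaps to face them and, after a short delay, spawns a BP_Bullet at its Arrow.
; Tick sets the player's collectible total to four and destroys the boss once that count is reached.
; Otherwise, after a delay, it opens Boss_Level if the player is below zero height.
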(event `self.ReceiveBeginPlay`
  (set `self.PlayerRef` (`GameplayStatics.GetPlayerCharacter` 0)))

(event `self.PawnSensing.OnSeePawn`
  (params (Pawn :type "Pawn Object Reference"))
  (cast `/Game/FirstPerson/Blueprints/BP_FirstPersonCharacter` Pawn)
  (`self.K2_SetActorRotation` (`KismetMathLibrary.FindLookAtRotation` (`self.K2_GetActorLocation`) (`self.K2_GetActorLocation` Pawn)))
  (`KismetSystemLibrary.Delay` 0.2)
  (`|SpawnActorFromClass` "/Game/MazeComponents/Blueprints/BP_Bullet.BP_Bullet_C" (`SceneComponent.K2_GetComponentToWorld` (`self.Arrow`)) "Undefined" "MultiplyWithRoot" null null))

(event `self.ReceiveTick`
  (params (DeltaSeconds :type "Float (single-precision)"))
  (bind (_returnvalue_x _returnvalue_y _returnvalue_z) (`KismetMathLibrary.BreakVector` (`self.K2_GetActorLocation` (`self.PlayerRef`))))
  (bind _asbp_first_person_character (cast `/Game/FirstPerson/Blueprints/BP_FirstPersonCharacter` (`self.PlayerRef`)))
  (set `/Game/FirstPerson/Blueprints/BP_FirstPersonCharacter.iTotalCollectibles` 4 _asbp_first_person_character)
  (if (>= (`/Game/FirstPerson/Blueprints/BP_FirstPersonCharacter.iCurrentCollectibles` _asbp_first_person_character) 4)
    (`self.K2_DestroyActor`)
    (else
      (`KismetSystemLibrary.Delay` 1.0)
      (if (< _returnvalue_z 0.0)
        (`GameplayStatics.OpenLevel` "Boss_Level")))))

(fn `UserConstructionScript`)