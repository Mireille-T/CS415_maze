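; Boss_Wall is a maze wall actor that periodically vanishes and reappears.
; From BeginPlay it waits for the Timer delay, plays a quiet laser sound at its location, then disables visibility, collision and tick.
; After a fixed two-second gap it restores all three and calls SpawnWall again, so the cycle loops indefinitely through self-recalling delays rather than a timer handle.
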(event `self.ReceiveBeginPlay`
  (`self.SpawnWall`))

(event `SpawnWall`
  (`KismetSystemLibrary.Delay` (`KismetMathLibrary.Conv_IntToDouble` (`self.Timer`)))
  (`GameplayStatics.PlaySoundAtLocation` "/Game/Audio/LaserCue.LaserCue" (`self.K2_GetActorLocation`) (struct) 0.1 1.0 0.0 null null null null)
  (`self.SetActorHiddenInGame` true)
  (`self.SetActorEnableCollision` false)
  (`self.SetActorTickEnabled` false)
  (`KismetSystemLibrary.Delay` 2.0)
  (`self.SetActorHiddenInGame` false)
  (`self.SetActorEnableCollision` true)
  (`self.SetActorTickEnabled` true)
  (`self.SpawnWall`))

(fn `UserConstructionScript`)