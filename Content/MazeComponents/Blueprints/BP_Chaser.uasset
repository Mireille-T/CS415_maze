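; BP_Chaser is a maze enemy pawn that wanders the level and chases the first-person player on sight.
; It roams by looping AIMoveTo to random reachable points around itself.
; PawnSensing sightings start a chase to the player's position and set a two-second recently-seen flag, which decides on arrival whether to chase again or resume roaming.
; Overlapping its Body2 component with the player opens Second_Maze_Level.
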(event `self.ReceiveBeginPlay`
  (`self.Roam`))

(event `Roam`
  (`|AIMoveTo` self (`NavigationSystemV1.K2_GetRandomReachablePointInRadius` (`self.K2_GetActorLocation`) 1000.0 null null) null
    (:`OnSuccess`
      (`KismetSystemLibrary.Delay` 0.2)
      (`self.Roam`))
    (:`OnFail`
      (`self.Roam`))))

(event `self.PawnSensing.OnSeePawn`
  (params (Pawn :type "Pawn Object Reference"))
  (cast `/Game/FirstPerson/Blueprints/BP_FirstPersonCharacter` Pawn)
  (`self.Chase`)
  (set `self.PawnSensedRecently` true)
  (`KismetSystemLibrary.Delay` 2.0)
  (set `self.PawnSensedRecently` false))

(event `Chase`
  (`|AIMoveTo` self (`self.K2_GetActorLocation` (`GameplayStatics.GetPlayerPawn` 0)) null
    (:`OnSuccess`
      (if (`self.PawnSensedRecently`)
        (`self.Chase`)
        (else
          (`self.Roam`))))))

(event `self.Body2.OnComponentBeginOverlap`
  (params (OverlappedComponent :type "PrimitiveComponent Object Reference") (OtherActor :type "Actor Object Reference") (OtherComp :type "PrimitiveComponent Object Reference") (OtherBodyIndex :type Integer) (bFromSweep :type Boolean) (SweepResult :type "HitResult Structure (by ref)"))
  (cast `/Game/FirstPerson/Blueprints/BP_FirstPersonCharacter` OtherActor)
  (`GameplayStatics.OpenLevel` "Second_Maze_Level"))

(fn `UserConstructionScript`)