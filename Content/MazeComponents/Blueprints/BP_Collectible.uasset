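; BP_Collectible is a maze pickup that the first-person player collects by walking into it.
; It starts at a random yaw, then spins each tick while its mesh bobs through a sine-driven local Z offset scaled by frequency and amplitude variables.
; When the Hitbox overlaps BP_FirstPersonCharacter, it increments that character's collectible count and destroys itself.
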(event `self.ReceiveBeginPlay`
  (`self.K2_SetActorRotation` (`KismetMathLibrary.MakeRotator` 0.0 0.0 (`KismetMathLibrary.RandomFloatInRange` 0.0 360.0))))

(event `self.ReceiveTick`
  (params (DeltaSeconds :type "Float (single-precision)"))
  (`self.K2_AddActorLocalRotation` (`KismetMathLibrary.MakeRotator` 0.0 0.0 (* DeltaSeconds (`self.fRotateSpeed`))))
  (`SceneComponent.K2_AddLocalOffset` (`self.StaticMeshComponent`) (`KismetMathLibrary.MakeVector` 0.0 0.0 (* (`KismetMathLibrary.Sin` (* (`self.GetGameTimeSinceCreation`) (`self.fFloatFrequency`))) (`self.fFloatAmplitude`))) false false))

(event `self.Hitbox.OnComponentBeginOverlap`
  (params (OverlappedComponent :type "PrimitiveComponent Object Reference") (OtherActor :type "Actor Object Reference") (OtherComp :type "PrimitiveComponent Object Reference") (OtherBodyIndex :type Integer) (bFromSweep :type Boolean) (SweepResult :type "HitResult Structure (by ref)"))
  (bind _asbp_first_person_character (cast `/Game/FirstPerson/Blueprints/BP_FirstPersonCharacter` OtherActor))
  (set `/Game/FirstPerson/Blueprints/BP_FirstPersonCharacter.iCurrentCollectibles` (+ (`/Game/FirstPerson/Blueprints/BP_FirstPersonCharacter.iCurrentCollectibles` _asbp_first_person_character) 1) _asbp_first_person_character)
  (`self.K2_DestroyActor`))

(fn `UserConstructionScript`)