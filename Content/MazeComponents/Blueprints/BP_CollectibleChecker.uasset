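; BP_CollectibleChecker is a maze exit that opens a portal once the player has gathered all collectibles.
; Overlapping its sphere compares the first-person character's collectible counts, then either shows an insufficient-collectibles text or reveals the portal and enables the capsule's overlap events.
; Entering that capsule loads Second_Maze_Level from First_Maze_Level, otherwise VictoryMenu.
; Tick yaws the text toward the player, spins the portal and bobs it on a sine wave.
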(event `self.ReceiveTick`
  (params (DeltaSeconds :type "Float (single-precision)"))
  (bind _portal (`self.Portal`))
  (bind (_returnvalue_roll _returnvalue_pitch _returnvalue_yaw) (`KismetMathLibrary.BreakRotator` (`KismetMathLibrary.FindLookAtRotation` (`self.K2_GetActorLocation`) (`self.K2_GetActorLocation` (`GameplayStatics.GetPlayerCharacter` 0)))))
  (`SceneComponent.K2_SetWorldRotation` (`self.Text_InsufficientCollectibles`) (`KismetMathLibrary.MakeRotator` 0.0 0.0 _returnvalue_yaw) false false)
  (`SceneComponent.K2_AddLocalRotation` _portal (`KismetMathLibrary.MakeRotator` 0.0 0.0 (* DeltaSeconds -16.0)) false false)
  (`SceneComponent.K2_AddLocalOffset` _portal (`KismetMathLibrary.MakeVector` 0.0 0.0 (* (`KismetMathLibrary.Sin` (* (`self.GetGameTimeSinceCreation`) 1.5)) 0.12)) false false))

(event `self.Sphere.OnComponentBeginOverlap`
  (params (OverlappedComponent :type "PrimitiveComponent Object Reference") (OtherActor :type "Actor Object Reference") (OtherComp :type "PrimitiveComponent Object Reference") (OtherBodyIndex :type Integer) (bFromSweep :type Boolean) (SweepResult :type "HitResult Structure (by ref)"))
  (bind _asbp_first_person_character (cast `/Game/FirstPerson/Blueprints/BP_FirstPersonCharacter` OtherActor))
  (if (< (`/Game/FirstPerson/Blueprints/BP_FirstPersonCharacter.iCurrentCollectibles` _asbp_first_person_character) (`/Game/FirstPerson/Blueprints/BP_FirstPersonCharacter.iTotalCollectibles` _asbp_first_person_character))
    (`SceneComponent.SetHiddenInGame` (`self.Text_InsufficientCollectibles`) false false)
    (else
      (`SceneComponent.SetHiddenInGame` (`self.Portal`) false false)
      (set `PrimitiveComponent.bGenerateOverlapEvents` true (`self.Capsule`)))))

(event `self.Sphere.OnComponentEndOverlap`
  (params (OverlappedComponent :type "PrimitiveComponent Object Reference") (OtherActor :type "Actor Object Reference") (OtherComp :type "PrimitiveComponent Object Reference") (OtherBodyIndex :type Integer))
  (cast `/Game/FirstPerson/Blueprints/BP_FirstPersonCharacter` OtherActor)
  (`SceneComponent.SetHiddenInGame` (`self.Text_InsufficientCollectibles`) true false))

(event `self.Capsule.OnComponentBeginOverlap`
  (params (OverlappedComponent :type "PrimitiveComponent Object Reference") (OtherActor :type "Actor Object Reference") (OtherComp :type "PrimitiveComponent Object Reference") (OtherBodyIndex :type Integer) (bFromSweep :type Boolean) (SweepResult :type "HitResult Structure (by ref)"))
  (cast `/Game/FirstPerson/Blueprints/BP_FirstPersonCharacter` OtherActor)
  (bind _returnvalue (`GameplayStatics.GetCurrentLevelName` true))
  (if (`KismetStringLibrary.EqualEqual_StrStr` _returnvalue "First_Maze_Level")
    (`GameplayStatics.OpenLevelBySoftObjectPtr` "/Game/MazeLevels/Second_Maze_Level.Second_Maze_Level")
    (else
      (`GameplayStatics.OpenLevelBySoftObjectPtr` "/Game/VictoryMenu.VictoryMenu"))))

(fn `UserConstructionScript`)