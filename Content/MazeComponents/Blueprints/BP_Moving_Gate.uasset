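; BP_Moving_Gate is a maze pawn that wanders on its own and toggles a CausesDeath flag as it relocates.
; It chains AI moves in random cardinal directions, retrying on failure and counting successes.
; Once the count exceeds MaxMovements, it clears the flag, waits a minute, then teleports to the next of three hard-coded locations.
; Shortly after teleporting, it sets the flag again and resumes wandering.
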(event `self.ReceiveBeginPlay`
  (`self.ChooseNewLocation`))

(event `ChooseNewLocation`
  (bind (_returnvalue_x _returnvalue_y _returnvalue_z) (`KismetMathLibrary.BreakVector` (`self.K2_GetActorLocation`)))
  (`|AIMoveTo` self (select `int` (`KismetMathLibrary.RandomIntegerInRange` 0 3) :`0` (`KismetMathLibrary.MakeVector` (+ _returnvalue_x 400.0) _returnvalue_y _returnvalue_z) :`1` (`KismetMathLibrary.MakeVector` (- _returnvalue_x 400.0) _returnvalue_y _returnvalue_z) :`2` (`KismetMathLibrary.MakeVector` _returnvalue_x (+ _returnvalue_y 400.0) _returnvalue_z) :`3` (`KismetMathLibrary.MakeVector` _returnvalue_x (- _returnvalue_y 400.0) _returnvalue_z) :!type "Vector Structure") null
    (:`OnSuccess`
      (set `self.MovementCount` (+ (`self.MovementCount`) 1))
      (if (> (`self.MovementCount`) (`self.MaxMovements`))
        (set `self.TeleportLocation` (mod (+ (`self.TeleportLocation`) 1) 3))
        (set `self.MovementCount` 0)
        (set `self.CausesDeath` false)
        (`KismetSystemLibrary.Delay` 60.0)
        (`self.Teleport`)
        (else
          (`self.ChooseNewLocation`))))
    (:`OnFail`
      (`self.ChooseNewLocation`))))

(event `Teleport`
  (`self.K2_SetActorLocation` (select `int` (`self.TeleportLocation`) :`0` (-100.0 2530.0 78.125) :`1` (-890.0 8880.0 78.125) :`2` (-823.0 12903.0 78.125) :!type "Vector Structure") false true)
  (`KismetSystemLibrary.Delay` 1.0)
  (set `self.CausesDeath` true)
  (`self.ChooseNewLocation`))

(fn `UserConstructionScript`)